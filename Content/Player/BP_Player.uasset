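; Player character Blueprint for a platformer with camera-relative movement, sprint, air jumps and a timed slide.
; Air jumps redirect horizontal speed along actor facing via LaunchCharacter and refill on landing; slides temporarily shrink the capsule and offset the mesh during a montage.
; It stores a checkpoint transform for respawns with a score penalty, updates the HUD score and opens the pause widget.
; Winning locks input, hides the HUD and saves score to the game instance.
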(event Custom|Respawn
  ;[0 0 0 1 35] Main features
  ;;[0 1 0.03793] Respawn to last Player Respawn Transform
  (Transformation|SetActorTransform (Variables|Player|GetPlayerRespawnTransform) false true)
  (CallFunction|ReduceScore (Variables|Score|GetDeathAmountScore)))

(event Custom|SetNewRespawnTransform
  (params (NewPlayerRespawnTransform :type Transform))
  ;[0 0 0 1 35] Main features
  ;;[0 1 0.03793] Set new respawn transform
  (Variables|Player|SetPlayerRespawnTransform NewPlayerRespawnTransform)
  ;;;[1 0.06771 0.06771] TODO Change checkpoint SFX
  (Audio|PlaySound2D "/Game/Imported/StarterContent/Audio/Explosion01.Explosion01" 1.0 1.0 0.0 0 0))

(event Custom|PlayerWon
  (bind _returnvalue (Game|GetPlayerController 0))
  ;[1 0.06771 0.06771] TODO Win condition
  (Default|CallPlayerHasWon)
  (Input|SetIgnoreMoveInput _returnvalue true)
  (Input|SetIgnoreLookInput _returnvalue true)
  (Widget|SetRenderOpacity (Variables|Widget|GetHUD_Ref) 0.0)
  (Default|SaveTotalScore (Variables|Score|GetGameInstanceRef) (Variables|Score|GetTotalScore)))

(event Custom|IncreaseScore
  (params (ScoreToAdd :type Integer))
  ;[0 0 0 1 35] Main features
  ;;[0 1 0.03793] Add score + display the score
  (bind _output_get (Variables|Score|SetTotalScore (+ ScoreToAdd (Variables|Score|GetTotalScore))))
  (Default|UpdateScore (Variables|Widget|GetHUD_Ref) _output_get))

(event Custom|ReduceScore
  (params (ScoreToSubstract :type Integer))
  ;[0 0 0 1 35] Main features
  ;;[0 1 0.03793] Substract X and set it to Total score + Update score to HUD
  (if (not (<= (Variables|Score|GetTotalScore) 0))
    (bind _output_get (Variables|Score|SetTotalScore (- (Variables|Score|GetTotalScore) ScoreToSubstract)))
    (Default|UpdateScore (Variables|Widget|GetHUD_Ref) _output_get)))

(event EventOnLanded
  (params (Hit :type Hit%20Result%20Structure%20%28by%20ref%29))
  ;[0.2055 1 0.2626] Jump & Double Jump
  (Variables|Default|SetCurrentJumps (Variables|Default|GetTotalJumps)))

(event EventBeginPlay
  (bind _returnvalue (Game|GetPlayerController 0))
  ;[0 0 0 1 35] Main features
  ;;[0 1 0.03793] BeginPlay: SaveCurrent transform to PlayerRespawnTransform + create hud
  (Variables|Player|SetPlayerRespawnTransform (Transformation|GetActorTransform))
  (Variables|Default|SetCurrentJumps (Variables|Default|GetTotalJumps))
  (bind _returnvalue_2 (UserInterface|CreateWidget "/Game/Blueprints/UI/WBP_Hud.WBP_Hud_C"))
  (bind _output_get (Variables|Widget|SetHUD_Ref _returnvalue_2))
  (UserInterface|Viewport|AddtoViewport _output_get 0)
  (Variables|/Script/Engine.PlayerController|SetbShowMouseCursor _returnvalue false)
  (Input|SetInputModeGameOnly _returnvalue false)
  (bind _asgi_my_game_instance (Utilities|Casting|CastToGI_MyGameInstance (Game|GetGameInstance)))
  (Variables|Score|SetGameInstanceRef _asgi_my_game_instance))

(event Input|ActionEvents|InputActionJump
  (params (Key :type Key%20Structure :default "None"))
  (bind _returnvalue (Transformation|GetActorForwardVector))
  (bind _charactermovement (Variables|Character|GetCharacterMovement))
  (bind _jumpzvelocity (Variables|/Script/Engine.CharacterMovementComponent|GetJumpZVelocity _charactermovement))
  (bind _velocity (Variables|/Script/Engine.MovementComponent|GetVelocity _charactermovement))
  (bind _returnvalue_2 (Math|Vector|MakeVector (.x _velocity) (.y _velocity) 0.0))
  (bind _returnvalue_3 (Math|Vector|VectorLength _returnvalue_2))
  (bind _returnvalue_4 (* _returnvalue _returnvalue_3))
  (bind _returnvalue_5 (Math|Vector|MakeVector (.x _returnvalue_4) (.y _returnvalue_4) _jumpzvelocity))
  ;[0.2055 1 0.2626] Jump & Double Jump
  (:Pressed
    (Character|Jump)
    (if (and (> (Variables|Default|GetCurrentJumps) 0) (AI|Components|NavMovement|IsFalling (Variables|Character|GetCharacterMovement)))
      (Variables|Default|SetCurrentJumps (- (Variables|Default|GetCurrentJumps) 1))
      (Character|LaunchCharacter (Math|Vector|MakeVector (.x _returnvalue_5) (.y _returnvalue_5) (.z _returnvalue_5)) true true)
      ;;[1 0.878 0.004132] Sound
      (Audio|PlaySound2D "/Engine/VREditor/Sounds/UI/Dockable_Window_Open.Dockable_Window_Open" 1.0 1.0 0.0 0 0)
      ;;[1 0 0] VFX
      (Effects|SpawnEmitteratLocation "/Game/Imported/StarterContent/Particles/P_Explosion.P_Explosion" (Transformation|GetActorLocation))))
  (:Released
    (Character|StopJumping)))

(event Input|ActionEvents|InputActionInGamePause
  (params (Key :type Key%20Structure :default "None"))
  ;[0 0 0] Widget
  ;;[0 1 0.03793] Create in game pause widget
  (:Pressed
    (bind _returnvalue (UserInterface|CreateWidget "/Game/Blueprints/UI/WBP_InGamePause.WBP_InGamePause_C"))
    (bind _output_get (Variables|Widget|SetInGamePauseRef _returnvalue))
    (UserInterface|Viewport|AddtoViewport _output_get 0)))

(event Input|ActionEvents|InputActionSlide
  (params (Key :type Key%20Structure :default "None"))
  (bind _charactermovement (Variables|Character|GetCharacterMovement))
  (bind _mesh (Variables|Character|GetMesh))
  (bind _mesh_2 (Variables|Character|GetMesh))
  ;[0.1784 1 0.3063] Sliding mechanic
  (:Pressed
    (if (and (> (Math|Vector|VectorLength (Variables|/Script/Engine.MovementComponent|GetVelocity _charactermovement)) 9e+01) (not (AI|Components|NavMovement|IsFalling _charactermovement)))
      (Utilities|FlowControl|DoOnce false :!label _label
        (:Completed
          (Components|Capsule|SetCapsuleHalfHeight (Variables|Collision|GetCapsuleComponent) 44.0 true)
          (Transformation|SetWorldLocation _mesh (+ (Transformation|GetWorldLocation _mesh) "0.000000,0.000000,40.000000") false false)
          (Animation|PlayAnimMontage "/Game/Player/Animations/SlidingDown_Montage.SlidingDown_Montage" 1.0 "None")
          (Utilities|FlowControl|Delay 1.0)
          (Components|Capsule|SetCapsuleHalfHeight (Variables|Collision|GetCapsuleComponent) 88.0 true)
          (Transformation|SetWorldLocation _mesh_2 (- (Transformation|GetWorldLocation _mesh_2) "0.000000,0.000000,40.000000") false false)
          (goto _label Reset))))))

(event Input|ActionEvents|InputActionSprint
  (params (Key :type Key%20Structure :default "None"))
  (bind _charactermovement (Variables|Character|GetCharacterMovement))
  ;[0.07268 1 0.1988] Input : Movement / Camera (mouse)
  (:Pressed
    (Variables|/Script/Engine.CharacterMovementComponent|SetMaxWalkSpeed _charactermovement 1e+03))
  (:Released
    (Variables|/Script/Engine.CharacterMovementComponent|SetMaxWalkSpeed _charactermovement 6e+02)))

(event Input|AxisEvents|InputAxisMoveForward/BackWard
  (params (AxisValue :type Float%20%28single-precision%29))
  ;[0.07268 1 0.1988] Input : Movement / Camera (mouse)
  (Pawn|Input|AddMovementInput (Math|Vector|GetForwardVector (Math|Rotator|MakeRotator 0.0 0.0 (.yaw (Pawn|GetControlRotation :!class /Script/Engine.Pawn)))) AxisValue false))

(event Input|AxisEvents|InputAxisMoveRight/Left
  (params (AxisValue :type Float%20%28single-precision%29))
  ;[0.07268 1 0.1988] Input : Movement / Camera (mouse)
  (Pawn|Input|AddMovementInput (Math|Vector|GetRightVector (Math|Rotator|MakeRotator 0.0 0.0 (.yaw (Pawn|GetControlRotation :!class /Script/Engine.Pawn)))) AxisValue false))

(event Input|AxisEvents|InputAxisMouseLook
  (params (AxisValue :type Float%20%28single-precision%29))
  ;[0.07268 1 0.1988] Input : Movement / Camera (mouse)
  (Pawn|Input|AddControllerYawInput AxisValue))

(event Input|AxisEvents|InputAxisMouseLookUp
  (params (AxisValue :type Float%20%28single-precision%29))
  ;[0.07268 1 0.1988] Input : Movement / Camera (mouse)
  (Pawn|Input|AddControllerPitchInput AxisValue))

(fn ConstructionScript)