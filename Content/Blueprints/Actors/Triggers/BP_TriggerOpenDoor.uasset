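; BP_TriggerOpenDoor is a trigger volume that opens a BP_ActivableDoor when every trigger of its class is activated.
; Box overlap sets its ActivatedKey, then scans all sibling triggers and opens the door found by class lookup if all are set.
; Ending overlap clears the key, closing the door only if that instance's own Open flag is set.
; Overlaps accept any actor and print debug values.
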(event OnComponentBeginOverlap(Box)
  (params (OverlappedComponent :type Primitive%20Component%20Object%20Reference) (OtherActor :type Actor%20Object%20Reference) (OtherComp :type Primitive%20Component%20Object%20Reference) (OtherBodyIndex :type Integer) (bFromSweep :type Boolean) (SweepResult :type Hit%20Result%20Structure%20%28by%20ref%29))
  (bind _output_get (Variables|Default|Setalltrue true))
  (Development|PrintString (Utilities|String|ToString(Boolean) _output_get))
  (Variables|Default|SetActivatedKey true)
  (bind _outactors (Actor|GetAllActorsOfClass "BP_TriggerOpenDoor_C"))
  (bind _array_element (Utilities|Array|ForEachLoopwithBreak _outactors :!label _label)
    (:LoopBody
      (if (not (Variables|BP_TriggerOpenDoor_C|GetActivatedKey _array_element))
        (bind _output_get_2 (Variables|Default|Setalltrue false))
        (Development|PrintString (Utilities|String|ToString(Boolean) _output_get_2))
        (goto _label Break)))
    (:Completed
      (if (Variables|Default|Getalltrue)
        (if (not (Variables|Default|Getopen))
          (bind _returnvalue (Actor|GetActorOfClass "/Game/Blueprints/Actors/BP_ActivableDoor.BP_ActivableDoor_C"))
          (Default|OpenDoor _returnvalue)
          (Variables|Default|Setopen true))
        (elif (Variables|Default|Getopen)
          (bind _returnvalue_2 (Actor|GetActorOfClass "/Game/Blueprints/Actors/BP_ActivableDoor.BP_ActivableDoor_C"))
          (Default|CloseDoor _returnvalue_2)
          (Variables|Default|Setopen false))))))

(event OnComponentEndOverlap(Box)
  (params (OverlappedComponent :type Primitive%20Component%20Object%20Reference) (OtherActor :type Actor%20Object%20Reference) (OtherComp :type Primitive%20Component%20Object%20Reference) (OtherBodyIndex :type Integer))
  (Variables|Default|SetActivatedKey false)
  (if (Variables|Default|Getopen)
    (bind _returnvalue (Actor|GetActorOfClass "/Game/Blueprints/Actors/BP_ActivableDoor.BP_ActivableDoor_C"))
    (Default|CloseDoor _returnvalue)
    (Variables|Default|Setopen false)))

(fn ConstructionScript)