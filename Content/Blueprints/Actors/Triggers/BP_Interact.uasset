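; BP_Interact is a trigger actor that lets the player interact with an arcade, which loads the MainMenu level.
; It creates a WBP_Interract prompt widget on BeginPlay.
; Overlapping the Box with the player character shows the prompt and arms an Interact flag, and leaving hides and clears it.
; The InteractWithArcade event opens the level only while that flag is set.
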(event OnComponentBeginOverlap(Box)
  (params (OverlappedComponent :type Primitive%20Component%20Object%20Reference) (OtherActor :type Actor%20Object%20Reference) (OtherComp :type Primitive%20Component%20Object%20Reference) (OtherBodyIndex :type Integer) (bFromSweep :type Boolean) (SweepResult :type Hit%20Result%20Structure%20%28by%20ref%29))
  (if (== OtherActor (Game|GetPlayerCharacter 0))
    (UserInterface|Viewport|AddtoViewport (Variables|Default|GetInteractWidget) 0)
    (Variables|Default|SetInteract true)))

(event OnComponentEndOverlap(Box)
  (params (OverlappedComponent :type Primitive%20Component%20Object%20Reference) (OtherActor :type Actor%20Object%20Reference) (OtherComp :type Primitive%20Component%20Object%20Reference) (OtherBodyIndex :type Integer))
  (if (== (Game|GetPlayerCharacter 0) OtherActor)
    (Widget|RemovefromParent (Variables|Default|GetInteractWidget))
    (Variables|Default|SetInteract false)))

(event Custom|InteractWithArcade
  (if (Variables|Default|GetInteract)
    (Game|OpenLevel(byName) "MainMenu")))

(event EventBeginPlay
  (bind _returnvalue (UserInterface|CreateWidget "/Game/Blueprints/UI/WBP_Interract.WBP_Interract_C"))
  (Variables|Default|SetInteractWidget _returnvalue))

(fn ConstructionScript)