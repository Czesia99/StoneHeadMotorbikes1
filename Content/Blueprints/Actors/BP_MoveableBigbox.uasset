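; BP_MoveableBigbox is a large box actor that the player can push.
; Separate X-axis and Y-axis collision components detect BP_Player overlaps, setting the player's IsPushing flag on entry and clearing it on exit.
; Both begin and end overlaps enable physics simulation on the Cube, and nothing in these graphs turns it off again.
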(event OnComponentBeginOverlap(YAxisCollision)
  (params (OverlappedComponent :type Primitive%20Component%20Object%20Reference) (OtherActor :type Actor%20Object%20Reference) (OtherComp :type Primitive%20Component%20Object%20Reference) (OtherBodyIndex :type Integer) (bFromSweep :type Boolean) (SweepResult :type Hit%20Result%20Structure%20%28by%20ref%29))
  ;[0.1456 1 0.3592] Y axis collision
  (bind _asbp_player (Utilities|Casting|CastToBP_Player OtherActor))
  (Physics|SetSimulatePhysics (Variables|Default|GetCube) true)
  (Variables|/Game/Player/BP_Player.BP_Player_C|SetIsPushing _asbp_player true))

(event OnComponentEndOverlap(YAxisCollision)
  (params (OverlappedComponent :type Primitive%20Component%20Object%20Reference) (OtherActor :type Actor%20Object%20Reference) (OtherComp :type Primitive%20Component%20Object%20Reference) (OtherBodyIndex :type Integer))
  ;[0.1456 1 0.3592] Y axis collision
  (bind _asbp_player (Utilities|Casting|CastToBP_Player OtherActor))
  (Physics|SetSimulatePhysics (Variables|Default|GetCube) true)
  (Variables|/Game/Player/BP_Player.BP_Player_C|SetIsPushing _asbp_player false))

(event OnComponentBeginOverlap(XAxisCollision1)
  (params (OverlappedComponent :type Primitive%20Component%20Object%20Reference) (OtherActor :type Actor%20Object%20Reference) (OtherComp :type Primitive%20Component%20Object%20Reference) (OtherBodyIndex :type Integer) (bFromSweep :type Boolean) (SweepResult :type Hit%20Result%20Structure%20%28by%20ref%29))
  ;[0.277 1 0.3519] X Axis collision
  (bind _asbp_player (Utilities|Casting|CastToBP_Player OtherActor))
  (Physics|SetSimulatePhysics (Variables|Default|GetCube) true)
  (Variables|/Game/Player/BP_Player.BP_Player_C|SetIsPushing _asbp_player true))

(event OnComponentEndOverlap(XAxisCollision1)
  (params (OverlappedComponent :type Primitive%20Component%20Object%20Reference) (OtherActor :type Actor%20Object%20Reference) (OtherComp :type Primitive%20Component%20Object%20Reference) (OtherBodyIndex :type Integer))
  ;[0.277 1 0.3519] X Axis collision
  (bind _asbp_player (Utilities|Casting|CastToBP_Player OtherActor))
  (Physics|SetSimulatePhysics (Variables|Default|GetCube) true)
  (Variables|/Game/Player/BP_Player.BP_Player_C|SetIsPushing _asbp_player false))

(fn ConstructionScript)