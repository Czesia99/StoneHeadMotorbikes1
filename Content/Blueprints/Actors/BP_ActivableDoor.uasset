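; BP_ActivableDoor is a door actor that opens and closes through OpenDoor and CloseDoor events, guarded by an Open flag.
; Each event fires the EventOpenDoor dispatcher, even when closing, then plays its own timeline to drive the mesh's relative Z location.
; The Open flag changes on timeline updates rather than when the animation finishes.
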(event Custom|CloseDoor
  (if (Variables|Default|GetOpen)
    (Default|CallEventOpenDoor)
    (bind _newtrack_0 (Timeline|Timeline_0 PlayFromStart)
      (:Update
        (Transformation|SetRelativeLocation (Variables|Default|GetStaticMesh) (Math|Vector|MakeVector 0.0 0.0 _newtrack_0) false false)
        (Variables|Default|SetOpen false)))))

(event Custom|OpenDoor
  (if (not (Variables|Default|GetOpen))
    (Default|CallEventOpenDoor)
    (bind _newtrack_0 (Timeline|Timeline PlayFromStart)
      (:Update
        (Transformation|SetRelativeLocation (Variables|Default|GetStaticMesh) (Math|Vector|MakeVector 0.0 0.0 _newtrack_0) false false)
        (Variables|Default|SetOpen true)))))

(fn ConstructionScript)