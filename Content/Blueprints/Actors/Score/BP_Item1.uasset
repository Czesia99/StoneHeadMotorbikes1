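; BP_Item1 is a score pickup that bobs vertically through a Timeline lerping between its start location and 50 units above.
; When BP_Player overlaps its sphere, it adds Score to the player, spawns confetti, plays an explosion sound and destroys itself.
; The random yaw and rotation-speed setup is disconnected and never runs, and a TODO marks the effects for replacement.
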(event OnComponentBeginOverlap(Sphere)
  (params (OverlappedComponent :type Primitive%20Component%20Object%20Reference) (OtherActor :type Actor%20Object%20Reference) (OtherComp :type Primitive%20Component%20Object%20Reference) (OtherBodyIndex :type Integer) (bFromSweep :type Boolean) (SweepResult :type Hit%20Result%20Structure%20%28by%20ref%29))
  ;[0 1 0.03793] Collision -> Increase score to player + destroy actor
  (bind _asbp_player (Utilities|Casting|CastToBP_Player OtherActor))
  (Default|IncreaseScore _asbp_player (Variables|Default|GetScore))
  ;;[1 0.06771 0.06771] TODO Change VFX + SFX
  (Niagara|SpawnSystematLocation "/Game/VFX/NS_Confetti_System.NS_Confetti_System" (Transformation|GetActorLocation) "0, 0, 0" "3.000000,3.000000,3.000000")
  (Audio|PlaySound2D "/Game/Imported/StarterContent/Audio/Explosion01.Explosion01" 1.0 1.0 0.0 0 0)
  (Actor|DestroyActor))

(event EventBeginPlay
  ;[0 1 0.03793] Begin play -> Set random rotation (Z:YAW) + Set random rotation speed (Z:YAW)
  (bind _output_get (Variables|Default|SetBaseLocation (Transformation|GetActorLocation)))
  (bind _newtrack_0 (Timeline|Timeline Play)
    (:Update
      (Transformation|SetRelativeLocation (Variables|Default|GetDefaultSceneRoot) (Math|Vector|Lerp(Vector) _output_get (+ _output_get "0.000000,0.000000,50.000000") _newtrack_0) false false))))

(fn ConstructionScript)