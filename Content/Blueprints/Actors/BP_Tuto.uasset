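; BP_Tuto is a spinning tutorial pickup that shows the player an info message when touched.
; On BeginPlay it takes a random yaw and gives its RotatingMovement component a random yaw spin rate.
; When the player character overlaps its Sphere, it creates a WBP_Tuto widget with its TutoInfoText, adds it to the viewport and destroys itself, so each instance triggers once.
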(event OnComponentBeginOverlap(Sphere)
  (params (OverlappedComponent :type Primitive%20Component%20Object%20Reference) (OtherActor :type Actor%20Object%20Reference) (OtherComp :type Primitive%20Component%20Object%20Reference) (OtherBodyIndex :type Integer) (bFromSweep :type Boolean) (SweepResult :type Hit%20Result%20Structure%20%28by%20ref%29))
  (if (== OtherActor (Game|GetPlayerCharacter 0))
    (bind _returnvalue (UserInterface|CreateWidget "/Game/Blueprints/Widgets/WBP_Tuto.WBP_Tuto_C" 0 (Variables|Default|GetTutoInfoText)))
    (UserInterface|Viewport|AddtoViewport _returnvalue 0)
    (Actor|DestroyActor)))

(event EventBeginPlay
  ;[0 1 0.03793] Begin play -> Set random rotation (Z:YAW) + Set random rotation speed (Z:YAW)
  (Transformation|SetActorRotation (Math|Rotator|MakeRotator 0.0 0.0 (Math|Random|RandomFloatinRange 0.0 1.8e+02)))
  (Variables|/Script/Engine.RotatingMovementComponent|SetRotationRate (Variables|Default|GetRotatingMovement) (Math|Rotator|MakeRotator 0.0 0.0 (Math|Random|RandomFloatinRange 1e+02 2e+02))))

(fn ConstructionScript)