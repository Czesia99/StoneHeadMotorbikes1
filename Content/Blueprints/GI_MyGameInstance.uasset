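; Game instance Blueprint that persists the player's best score in a save slot.
; SaveTotalScore loads the existing SG_BestScore save, or creates one seeded with the incoming score when none exists, then writes it back to the slot.
; CheckIfBestScoreIsBetter keeps the higher of stored and new scores, comparing against the NewScoreToTest variable rather than its own input.
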(event Custom|SaveTotalScore
  (params (ScoreToSave :type Integer))
  (Variables|Default|SetNewScoreToTest ScoreToSave)
  (bind _returnvalue (SaveGame|DoesSaveGameExist (Variables|Default|GetSlotName)))
  (if _returnvalue
    (bind _returnvalue_2 (SaveGame|LoadGamefromSlot (Variables|Default|GetSlotName)))
    (bind _assg_best_score (Utilities|Casting|CastToSG_BestScore _returnvalue_2))
    (bind _scoretosave (Utilities|CheckifBestScoreIsBetter (Variables|/Game/Blueprints/SG_BestScore.SG_BestScore_C|GetBestScore _assg_best_score) (Variables|Default|GetNewScoreToTest))
      (:Exec
        (Variables|/Game/Blueprints/SG_BestScore.SG_BestScore_C|SetBestScore _assg_best_score _scoretosave)
        (Variables|Default|SetSaveGameRef _assg_best_score)))
    (else
      (bind _returnvalue_3 (SaveGame|CreateSaveGameObject "/Game/Blueprints/SG_BestScore.SG_BestScore_C"))
      (Variables|/Game/Blueprints/SG_BestScore.SG_BestScore_C|SetBestScore _returnvalue_3 (Variables|Default|GetNewScoreToTest))
      (Variables|Default|SetSaveGameRef _returnvalue_3)))
  (SaveGame|SaveGametoSlot (Variables|Default|GetSaveGameRef) (Variables|Default|GetSlotName)))