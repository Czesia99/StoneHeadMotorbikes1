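; BP_LateralStabilizer is a component that resists sideways sliding of the physics body it belongs to, in the PlayerCar folder.
; On BeginPlay it caches the owner's root as a primitive component.
; Each Tick it projects that body's linear velocity onto its right vector and applies an opposing force along that axis, scaled by SpeedToForceFactor, without compensating for mass.
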(event EventBeginPlay
  ;[0.2837 1 0.4135] GET COMPONENT
  (bind _asprimitive_component (Utilities|Casting|CastToPrimitiveComponent (Variables|/Script/Engine.Actor|GetRootComponent (Components|GetOwner))))
  (Variables|Default|SetRefToBody _asprimitive_component))

(event EventTick
  (params (DeltaSeconds :type Float%20%28single-precision%29))
  (bind _reftobody (Variables|Default|GetRefToBody))
  (bind _reftobody_2 (Variables|Default|GetRefToBody)
    (:then
      (bind _returnvalue (Physics|GetPhysicsLinearVelocity _reftobody_2 "None"))
      (Physics|AddForce _reftobody (* (* (Math|Vector|DotProduct _returnvalue (Math|Vector|GetRightVector _reftobody_2)) -1.0 (Variables|Default|GetSpeedToForceFactor)) (Math|Vector|GetRightVector _reftobody)) "None" false))
    (:else)))