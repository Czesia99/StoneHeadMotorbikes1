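; BP_Speedcar3 is a player-driven car that passes input to its MovementComponent and can right itself when flipped.
; Forward input, scaled by acceleration and a Sprint boost, sets target speed; steering sets target angular speed, reversing with the forward input's sign.
; Mouse look rotates the SpringArm camera.
; Jump, when the body is upside down, launches it with an impulse, then rolls it with a delayed angular impulse.
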(event EventBeginPlay)

(event Collision|EventActorBeginOverlap
  (params (OtherActor :type Actor%20Object%20Reference)))

(event EventTick
  (params (DeltaSeconds :type Float%20%28single-precision%29)))

(event Input|ActionEvents|InputActionSprint
  (params (Key :type Key%20Structure :default "None"))
  (:Pressed
    (Variables|Default|SetBoostMultplier 3.0))
  (:Released
    (Variables|Default|SetBoostMultplier 1.0)))

(event Input|ActionEvents|InputActionJump
  (params (Key :type Key%20Structure :default "None"))
  (bind _body (Variables|Default|GetBody))
  (bind _body_2 (Variables|Default|GetBody))
  (:Pressed
    (if (< (Math|Vector|DotProduct (Math|Vector|GetUpVector (Variables|Default|GetBody)) (Math|Vector|MakeVector 0.0 0.0 1.0)) -0.2)
      (Physics|AddImpulse _body (* (Math|Vector|GetUpVector _body) -6.5e+05) "None" false)
      (Utilities|FlowControl|Delay 0.2)
      (Class|PrimitiveComponent|AddAngularImpulseinDegrees _body_2 (* (Math|Vector|GetForwardVector _body_2) 8e+08) "None" false))))

(event Input|AxisEvents|InputAxisMouseLookUp
  (params (AxisValue :type Float%20%28single-precision%29))
  (Transformation|AddRelativeRotation (Variables|Default|GetSpringArm) (Math|Rotator|MakeRotator 0.0 AxisValue 0.0) false false))

(event Input|AxisEvents|InputAxisMouseLook
  (params (AxisValue :type Float%20%28single-precision%29))
  (Transformation|AddRelativeRotation (Variables|Default|GetSpringArm) (Math|Rotator|MakeRotator 0.0 0.0 AxisValue) false false))

(event Input|AxisEvents|InputAxisMoveForward/BackWard
  (params (AxisValue :type Float%20%28single-precision%29))
  (Variables|/Game/PlayerCar/BP_MovementComponent.BP_MovementComponent_C|SetTargetSpeed (Variables|Default|GetMovementComponent) (* AxisValue (Variables|Default|Getacceleration) (Variables|Default|GetBoostMultplier))))

(event Input|AxisEvents|InputAxisMoveRight/Left
  (params (AxisValue :type Float%20%28single-precision%29))
  (bind _returnvalue (Input|AxisValues|GetMoveForward/BackWard))
  (Development|PrintText (Utilities|Text|ToText(Float) AxisValue "HalfToEven"))
  (Variables|/Game/PlayerCar/BP_MovementComponent.BP_MovementComponent_C|SetTargetAngularSpeed (Variables|Default|GetMovementComponent) (* AxisValue 1e+02 (select (== _returnvalue 0.0) 1.0 (Math|Float|Sign(Float) _returnvalue)))))

(fn ConstructionScript)